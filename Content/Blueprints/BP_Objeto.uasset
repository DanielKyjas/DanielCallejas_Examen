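; BP_Objeto is a findable object that the first-person player collects by walking into its box trigger.
; On begin play it hides the FoundIt element by tinting it transparent.
; When BP_FirstPersonCharacter overlaps the box, it destroys the static mesh and box components, then fades out the Find element and shows FoundIt by swapping their tint opacity.
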(event OnComponentBeginOverlap(Box)
  (params (OverlappedComponent :type Primitive%20Component%20Object%20Reference) (OtherActor :type Actor%20Object%20Reference) (OtherComp :type Primitive%20Component%20Object%20Reference) (OtherBodyIndex :type Integer) (bFromSweep :type Boolean) (SweepResult :type Hit%20Result%20Structure%20%28by%20ref%29))
  (Utilities|Casting|CastToBP_FirstPersonCharacter OtherActor)
  (Components|DestroyComponent (Variables|Default|GetStaticMesh))
  (Components|DestroyComponent (Variables|Default|GetBox))
  (Class|WidgetComponent|SetTintColorandOpacity (Variables|Default|GetFind) "(R=1.000000,G=1.000000,B=1.000000,A=0.000000)")
  (Class|WidgetComponent|SetTintColorandOpacity (Variables|Default|GetFoundIt) "(R=1.000000,G=1.000000,B=1.000000,A=1.000000)"))

(event EventBeginPlay
  (Class|WidgetComponent|SetTintColorandOpacity (Variables|Default|GetFoundIt) "(R=0.000000,G=0.000000,B=0.000000,A=0.000000)"))

(event Collision|EventActorBeginOverlap
  (params (OtherActor :type Actor%20Object%20Reference)))

(event EventTick
  (params (DeltaSeconds :type Float%20%28single-precision%29)))

(fn ConstructionScript)